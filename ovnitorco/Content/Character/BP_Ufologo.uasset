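; BP_Ufologo is a player-controlled character that moves on the world X and Y axes through Enhanced Input.
; BeginPlay adds the IMC_Ovnitorco mapping context, and IA_Movimiento stores the input in Dirección and feeds it to AddMovementInput.
; Tick prints the length of Velocidad as debug output, though nothing here sets that variable.
; An unconnected branch that casts the player controller to WBP_Menu and adds it to the viewport never runs.
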(event `self.ReceiveBeginPlay`
  (bind _asplayer_controller (cast `PlayerController` (`self.GetController`)))
  (`EnhancedInputSubsystemInterface.AddMappingContext` (pcsubsystem `EnhancedInputLocalPlayerSubsystem` _asplayer_controller) "/Game/IMC_Ovnitorco.IMC_Ovnitorco" 0 (struct)))

(event `self.ReceiveTick`
  (params (DeltaSeconds :type "Float (single-precision)"))
  (`KismetSystemLibrary.PrintString` (`KismetStringLibrary.Conv_DoubleToString` (`KismetMathLibrary.VSize` (`self.Velocidad`))) true true (struct :`G` 0.66 :`B` 1.0 :`A` 1.0) 0.1))

(event `EnhancedInput|/Game/Imputs/IA_Movimiento`
  (params (ActionValue :type "Vector2D Structure") (ElapsedSeconds :type "Float (double-precision)") (TriggeredSeconds :type "Float (double-precision)") (InputAction :type "InputAction Object Reference" :default "/Game/Imputs/IA_Movimiento.IA_Movimiento"))
  (bind (_x _y) (`KismetMathLibrary.BreakVector2D` ActionValue))
  (:`Triggered`
    (set `self.Dirección` ActionValue)
    (`self.AddMovementInput` (1.0 0.0 0.0) _x)
    (`self.AddMovementInput` (0.0 1.0 0.0) _y)))

(event `EnhancedInput|/Game/Imputs/IA_Menu`
  (params (ActionValue :type Boolean) (ElapsedSeconds :type "Float (double-precision)") (TriggeredSeconds :type "Float (double-precision)") (InputAction :type "InputAction Object Reference" :default "/Game/Imputs/IA_Menu.IA_Menu")))

(fn `UserConstructionScript`)