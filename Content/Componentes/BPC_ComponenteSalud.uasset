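; Health component that tracks an actor's life for damage handling.
; DisminuirVida subtracts the incoming damage from Vida, clamps it between 0 and 100, and fires the SeBajóLavida dispatcher with current and maximum life.
; It prints the new value and a death message when life reaches zero; death has no other effect here, and the clamp ignores VidaMaxima.
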(fn `DisminuirVida`
  (params (`Daño` :type "Float (double-precision)"))
  (bind _output_get (set `self.Vida` (`KismetMathLibrary.FClamp` (- (`self.Vida`) `Daño`) 0.0 100.0)))
  (`self.SeBajóLavida` (`self.Vida`) (`self.VidaMaxima`))
  (`KismetSystemLibrary.PrintString` (`KismetStringLibrary.Conv_DoubleToString` _output_get))
  (if (<= _output_get 0.0)
    (`KismetSystemLibrary.PrintString` "esta muerto")))