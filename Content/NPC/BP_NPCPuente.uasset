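; BP_NPCPuente is an NPC actor that offers a line-by-line dialogue when something enters its Box trigger.
; Overlap shows a TextRender and creates the WBP_Dialogo widget; leaving hides the text and removes the widget.
; The Dialogo event, not called within this Blueprint, passes TextosDialogos to the widget, then advances its line index or removes it after the last line.
; A DoOnce gates Dialogo but resets immediately; player input toggling is unconnected.
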(event `self.Box.OnComponentBeginOverlap`
  (params (OverlappedComponent :type "PrimitiveComponent Object Reference") (OtherActor :type "Actor Object Reference") (OtherComp :type "PrimitiveComponent Object Reference") (OtherBodyIndex :type Integer) (bFromSweep :type Boolean) (SweepResult :type "HitResult Structure (by ref)"))
  (`SceneComponent.SetHiddenInGame` (`self.Text Render`) false false)
  (bind _returnvalue (`|CreateWidget` "/Game/Widget/Historia/WBP_Dialogo.WBP_Dialogo_C"))
  (bind _output_get (set `self.DialogosWidget` _returnvalue))
  (`UserWidget.AddToViewport` _output_get 0))

(event `self.Box.OnComponentEndOverlap`
  (params (OverlappedComponent :type "PrimitiveComponent Object Reference") (OtherActor :type "Actor Object Reference") (OtherComp :type "PrimitiveComponent Object Reference") (OtherBodyIndex :type Integer))
  (bind _dialogoswidget (`self.DialogosWidget`))
  (`SceneComponent.SetHiddenInGame` (`self.Text Render`) true false)
  (`/Engine/EditorBlueprintResources/StandardMacros.IsValid` _dialogoswidget
    (:`Is Valid`
      (`Widget.RemoveFromParent` _dialogoswidget))))

(event `/Game/Interfases/BPI_Dialogos.Dialogo`
  (bind _dialogoswidget (`self.DialogosWidget`))
  (bind _dialogoswidget_2 (`self.DialogosWidget`))
  (bind _returnvalue (+ (`/Game/Widget/Historia/WBP_Dialogo.LineaDeTexto` (`self.DialogosWidget`)) 1))
  (`/Engine/EditorBlueprintResources/StandardMacros.DoOnce` false :!label _label
    (:`Completed`
      (set `/Game/Widget/Historia/WBP_Dialogo.TextosDialogos` (`self.Textos Dialogos`) _dialogoswidget_2)
      (`Widget.SetVisibility` (`/Game/Widget/Historia/WBP_Dialogo.TextoDialogos` _dialogoswidget_2) "Visible")
      (`Widget.SetVisibility` (`/Game/Widget/Historia/WBP_Dialogo.Fondodialogo` _dialogoswidget_2) "Visible")
      (if (> _returnvalue (- (`KismetArrayLibrary.Array_Length` (`self.Textos Dialogos`)) 1))
        (`Widget.RemoveFromParent` _dialogoswidget)
        (`self.Resetdoonce`)
        (else
          (set `/Game/Widget/Historia/WBP_Dialogo.LineaDeTexto` _returnvalue _dialogoswidget)
          (`self.Resetdoonce`))))))

(event `Resetdoonce`
  (goto _label :!via `Reset`))

(fn `UserConstructionScript`)