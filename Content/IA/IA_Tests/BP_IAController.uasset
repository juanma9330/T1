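; Test AI controller that runs the BP_AIArbol behavior tree on possession and feeds it a perceived enemy target.
; Perception updates that cast to BP_Ufologo set the TargetEnemigo blackboard key to that actor when sensed, and clear it when sensing fails.
; Debug strings report when the enemy is seen or lost.
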(event `self.ReceivePossess`
  (params (PossessedPawn :type "Pawn Object Reference"))
  (`self.RunBehaviorTree` "/Game/IA/IA_Tests/BP_AIArbol.BP_AIArbol"))

(event `self.AIPerception.OnTargetPerceptionUpdated`
  (params (Actor :type "Actor Object Reference") (Stimulus :type "AIStimulus Structure"))
  (bind _asbp_ufologo (cast `/Game/Character/BP_Ufologo` Actor))
  (if Stimulus_bSuccessfullySensed
    (`BlackboardComponent.SetValueAsObject` (`AIBlueprintHelperLibrary.GetBlackboard` null) (`self.TargetEnemigo`) _asbp_ufologo)
    (`KismetSystemLibrary.PrintString` "ViAlEnemigo")
    (else
      (`BlackboardComponent.SetValueAsObject` (`AIBlueprintHelperLibrary.GetBlackboard` null) (`self.TargetEnemigo`) null)
      (`KismetSystemLibrary.PrintString` "LoPerdí de vista"))))

(fn `UserConstructionScript`)