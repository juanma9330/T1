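; BP_Prueba is a test actor in the boss folder that turns Niagara particle callbacks into damage.
; On BeginPlay it registers itself as the Niagara component's BPNiagaraCallback object.
; Each particle data callback applies fixed damage to Target without reading the particle data.
; An unconnected loop that would sphere-trace along each particle's velocity and damage the hit actor never runs.
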(event `self.ReceiveBeginPlay`
  (`NiagaraComponent.SetVariableObject` (`self.Niagara`) "BPNiagaraCallback" self))

(event `self.ReceiveParticleData`
  (params (Data :type "Array of BasicParticleData Structure (by ref)") (NiagaraSystem :type "NiagaraSystem Object Reference") (SimulationPositionOffset :type "Vector Structure (by ref)"))
  (`GameplayStatics.ApplyDamage` (`self.Target`) 2.0))

(fn `UserConstructionScript`)