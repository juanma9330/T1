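; Projectile for the boss's ranged attack, moving by a swept local offset on X and Y every tick.
; Sphere overlap deals configurable damage to the overlapped actor and destroys the projectile.
; A Niagara effect also deals fixed damage to a stored Target through component overlap and a particle-data callback event.
; Homing direction math and radial flipbook spawning are present but never run.
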(event `self.ReceiveBeginPlay`
  (`NiagaraComponent.SetVariableObject` (`self.FX_Boss`) "BPNiagaraCallback" null))

(event `self.Sphere.OnComponentBeginOverlap`
  (params (OverlappedComponent :type "PrimitiveComponent Object Reference") (OtherActor :type "Actor Object Reference") (OtherComp :type "PrimitiveComponent Object Reference") (OtherBodyIndex :type Integer) (bFromSweep :type Boolean) (SweepResult :type "HitResult Structure (by ref)"))
  (`GameplayStatics.ApplyDamage` OtherActor (`self.Daño`))
  (`KismetSystemLibrary.PrintString` "ataque aguijon")
  (`self.K2_DestroyActor`))

(event `self.ReceiveTick`
  (params (DeltaSeconds :type "Float (single-precision)"))
  (bind _velocidaddebala (`self.Velocidaddebala`))
  (`self.K2_AddActorLocalOffset` (`KismetMathLibrary.MakeVector` _velocidaddebala _velocidaddebala) true))

(event `self.FX_Boss.OnComponentBeginOverlap`
  (params (OverlappedComponent :type "PrimitiveComponent Object Reference") (OtherActor :type "Actor Object Reference") (OtherComp :type "PrimitiveComponent Object Reference") (OtherBodyIndex :type Integer) (bFromSweep :type Boolean) (SweepResult :type "HitResult Structure (by ref)"))
  (`GameplayStatics.ApplyDamage` (`self.target`) 3.0))

(event `self.ReceiveParticleData`
  (params (Data :type "Array of BasicParticleData Structure (by ref)") (NiagaraSystem :type "NiagaraSystem Object Reference") (SimulationPositionOffset :type "Vector Structure (by ref)"))
  (`KismetSystemLibrary.PrintString` "Hello")
  (`GameplayStatics.ApplyDamage` (`self.target`) 4.0))

(fn `UserConstructionScript`)