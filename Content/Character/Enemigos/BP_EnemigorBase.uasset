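; BP_EnemigorBase is the base enemy Blueprint, providing attack, targeting and death events.
; AtaqueEnemigo plays the PaperZD-style mummy attack override animation, using EstáAtacando to block re-entry until it completes or is cancelled.
; ObjetivoDeAtaque writes the given target into the AI controller's Blackboard.
; Muerte destroys the actor when flagged dead; all three events print debug messages.
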(event `self.ReceiveBeginPlay`
  (`parent.ReceiveBeginPlay`))

(event `/Game/Interfases/BPI_AtaqueEnmigo.AtaqueEnemigo`
  (if (not (`self.EstáAtacando?`))
    (`PaperZDPlaySlotOverrideAction.PlayAnimationOverrideWithCallbacks` (`PaperZDAnimationComponent.AnimInstance` (`self.AnimationComponent`)) "/Game/Character/Enemigos/EnemigoMelé/Animaciones/AnimSequences/AtaqueMomia.AtaqueMomia"
      (:`then`
        (set `self.EstáAtacando?` true)
        (`KismetSystemLibrary.PrintString` "ATAQUE ENMIGO" true true (struct :`R` 1.0 :`G` 0.383758 :`A` 1.0)))
      (:`OnCompleted`
        (set `self.EstáAtacando?` false :!label _label))
      (:`OnCancelled`
        (goto _label)))))

(event `/Game/Interfases/BPI_AtaqueEnmigo.ObjetivoDeAtaque`
  (params (Objetivo :type "/Game/Character/animaciones_Ufologo/ABP_Ufologo Object Reference"))
  (bind _returnvalue (`AIBlueprintHelperLibrary.GetBlackboard` (`self.GetController`)))
  (`BlackboardComponent.SetValueAsObject` _returnvalue (`self.BBKey_Target`) Objetivo)
  (`KismetSystemLibrary.PrintString` (`KismetSystemLibrary.GetDisplayName` _returnvalue)))

(event `self.Muerte`
  (params (Vida :type "Float (double-precision)") (`EstáMuerto?` :type Boolean))
  (if `EstáMuerto?`
    (`self.K2_DestroyActor`)
    (`KismetSystemLibrary.PrintString` "enemigomuerto" true true (struct :`R` 1.0 :`G` 0.049568 :`B` 0.199456 :`A` 1.0))))

(fn `UserConstructionScript`)