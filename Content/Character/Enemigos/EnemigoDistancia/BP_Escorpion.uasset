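; BP_Escorpion is a scorpion enemy, filed under ranged enemies, that extends a parent class and damages actors it touches.
; Overlaps on HitboxEnemiga apply BaseDamage and overlaps on BoxAtaque apply DañoMele, with no filter on the other actor.
; Health events set and update a WBP_VidaEnemigo bar on its Widget component, and the actor is destroyed at zero health.
; AtaqueEnemigo is an empty stub still awaiting animation.
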(event `self.ReceiveBeginPlay`
  (`parent.ReceiveBeginPlay`))

(event `self.HitboxEnemiga.OnComponentBeginOverlap`
  (params (OverlappedComponent :type "PrimitiveComponent Object Reference") (OtherActor :type "Actor Object Reference") (OtherComp :type "PrimitiveComponent Object Reference") (OtherBodyIndex :type Integer) (bFromSweep :type Boolean) (SweepResult :type "HitResult Structure (by ref)"))
  (`GameplayStatics.ApplyDamage` OtherActor (`self.Base Damage`)))

(event `self.ReceiveActorBeginOverlap`
  (params (OtherActor :type "Actor Object Reference")))

(event `/Game/Character/BP_CharacterBase.VidaAlIniciar`
  (params (Vida :type "Float (double-precision)") (VidaMaxima :type "Float (double-precision)"))
  (bind _aswbp_vida_enemigo (cast `/Game/UI/BarraVidaEnemigo/WBP_VidaEnemigo` (`WidgetComponent.GetWidget` (`self.Widget`))))
  (set `self.As WBP Vida Enemigo` _aswbp_vida_enemigo)
  (`self.ActualizarVidaInicialWidget` Vida VidaMaxima))

(event `/Game/Character/BP_CharacterBase.alertaDaño`
  (params (Vida :type "Float (double-precision)") (VidaMaxima :type "Float (double-precision)"))
  (bind _aswbp_vida_enemigo (cast `/Game/UI/BarraVidaEnemigo/WBP_VidaEnemigo` (`WidgetComponent.GetWidget` (`self.Widget`))))
  (bind _output_get (set `self.As WBP Vida Enemigo` _aswbp_vida_enemigo))
  (`/Game/UI/BarraVidaEnemigo/WBP_VidaEnemigo.ActualizarBarraEnemigo` _output_get Vida VidaMaxima)
  (if (<= Vida 0.0)
    (`self.K2_DestroyActor`)))

(event `self.AtaqueEnemigo`
  ;[1 1 1] Falta animación
)

(event `self.BoxAtaque.OnComponentBeginOverlap`
  (params (OverlappedComponent :type "PrimitiveComponent Object Reference") (OtherActor :type "Actor Object Reference") (OtherComp :type "PrimitiveComponent Object Reference") (OtherBodyIndex :type Integer) (bFromSweep :type Boolean) (SweepResult :type "HitResult Structure (by ref)"))
  (`GameplayStatics.ApplyDamage` OtherActor (`self.DañoMele`)))

(fn `ActualizarVidaInicialWidget`
  (params (Vida :type "Float (double-precision)") (`vidaMáx` :type "Float (double-precision)"))
  (`ProgressBar.SetPercent` (`/Game/UI/BarraVidaEnemigo/WBP_VidaEnemigo.BarraVidaEnemigo` (`self.As WBP Vida Enemigo`)) (/ Vida `vidaMáx`)))

(fn `UserConstructionScript`)