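; Player character Ufologo, a PaperZD sprite pawn with Enhanced Input movement, sprint, dash, melee and arrow attacks, interaction and coin/gem pickup counters.
; Dash disables collision and gravity, then snaps to a line-trace hit or launches forward on a cooldown.
; Animation overrides gate attack states, with Espadazo damaging enemies overlapping HitBox.
; Health events update WBP_HUD, while debug keys M/N save and restore through BP_GIPlayer, applying only the saved transform.
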(event Custom|termino%20el%20dash
  ;[1 1 1] Dash
  (Variables|/Script/Engine.CharacterMovementComponent|SetGravityScale (Variables|Character|GetCharacterMovement) 1.0)
  (Collision|SetCollisionEnabled (Variables|Default|GetCapsuleComponent) "QueryAndPhysics")
  (Utilities|Time|ClearTimerbyFunctionName 0 "termino el dash"))

(event Input|EnhancedActionEvents|EnhancedInputActionIA_Movimiento
  (params (ActionValue :type Vector%202D%20Structure) (ElapsedSeconds :type Float%20%28double-precision%29) (TriggeredSeconds :type Float%20%28double-precision%29) (InputAction :type Input%20Action%20Object%20Reference :default "/Game/Imputs/IA_Movimiento.IA_Movimiento"))
  (bind (_x _y) (Math|Vector2D|BreakVector2D ActionValue))
  ;[1 1 1] Movimiento
  (if (not (Variables|Default|GetEstáAtacando?))
    (if (not (Variables|Default|GetEstaDisparando))
      (Variables|Default|SetDirección ActionValue)
      (Pawn|Input|AddMovementInput "1.000000,0.000000,0.000000" _x false)
      (Pawn|Input|AddMovementInput "0.000000,1.000000,0.000000" _y false))))

(event Input|EnhancedActionEvents|EnhancedInputActionIA_Interacuar
  (params (ActionValue :type Boolean) (ElapsedSeconds :type Float%20%28double-precision%29) (TriggeredSeconds :type Float%20%28double-precision%29) (InputAction :type Input%20Action%20Object%20Reference :default "/Game/Imputs/IA_Interacuar.IA_Interacuar"))
  (:Triggered
    (CallFunction|Interactuar)))

(event Input|EnhancedActionEvents|EnhancedInputActionIA_Correr
  (params (ActionValue :type Boolean) (ElapsedSeconds :type Float%20%28double-precision%29) (TriggeredSeconds :type Float%20%28double-precision%29) (InputAction :type Input%20Action%20Object%20Reference :default "/Game/Imputs/IA_Correr.IA_Correr"))
  (bind _charactermovement (Variables|Character|GetCharacterMovement))
  ;[1 1 1] Correr
  (:Started
    (Variables|/Script/Engine.CharacterMovementComponent|SetMaxWalkSpeed _charactermovement (* (Variables|/Script/Engine.CharacterMovementComponent|GetMaxWalkSpeed _charactermovement) 3.0)))
  (:Completed
    (Variables|/Script/Engine.CharacterMovementComponent|SetMaxWalkSpeed _charactermovement 6e+02)))

(event Input|EnhancedActionEvents|EnhancedInputActionIA_Dash
  (params (ActionValue :type Boolean) (ElapsedSeconds :type Float%20%28double-precision%29) (TriggeredSeconds :type Float%20%28double-precision%29) (InputAction :type Input%20Action%20Object%20Reference :default "/Game/Imputs/IA_Dash.IA_Dash"))
  (bind _returnvalue (Transformation|GetActorLocation))
  (bind _returnvalue_2 (Transformation|GetActorForwardVector))
  (bind _veldash (Variables|Default|Getveldash))
  (bind _returnvalue_3 (* _returnvalue_2 _veldash))
  ;[1 1 1] Dash
  (:Started
    (if (not (Variables|Default|GetEstáAtacando?))
      (if (not (Variables|Default|GetEstaDisparando))
        (if (Variables|Default|GetPuedoHacerDash?)
          (Variables|Default|SetPuedoHacerDash? false)
          (Collision|SetCollisionEnabled (Variables|Default|GetCapsuleComponent) "NoCollision")
          (Variables|/Script/Engine.CharacterMovementComponent|SetGravityScale (Variables|Character|GetCharacterMovement) 0.0)
          (bind (_outhit _returnvalue_4) (Collision|LineTraceForObjects _returnvalue (+ _returnvalue (Math|Vector|MakeVector (.x _returnvalue_3) (.y _returnvalue_3) 0.0)) (Utilities|Array|MakeArray "ObjectTypeQuery1" "ObjectTypeQuery2") false 0 "Persistent"))
          (if _returnvalue_4
            (Transformation|SetActorLocation (.ImpactPoint (Collision|BreakHitResult _outhit)) (.bBlockingHit (Collision|BreakHitResult _outhit)) false)
            (else
              (Character|LaunchCharacter (* (Transformation|GetActorForwardVector) (Variables|Default|GetVelocidad%20Dash)) true false)))
          (Utilities|Time|SetTimerbyEvent (delegate Custom|termino%20el%20dash) (Variables|Default|GetDuracionDash))
          (Utilities|FlowControl|Delay (Variables|Default|GetRecargaDash))
          (Variables|Default|SetPuedoHacerDash? true))))))

(event Input|EnhancedActionEvents|EnhancedInputActionIA_AtaqueMele
  (params (ActionValue :type Boolean) (ElapsedSeconds :type Float%20%28double-precision%29) (TriggeredSeconds :type Float%20%28double-precision%29) (InputAction :type Input%20Action%20Object%20Reference :default "/Game/Imputs/IA_AtaqueMele.IA_AtaqueMele"))
  ;[1 1 1] ataque mele
  (if (not (Variables|Default|GetEstáAtacando?))
    (|PlayAnimationOverridewithCallbacks (Variables|/Script/PaperZD.PaperZDAnimationComponent|GetAnimInstance (Variables|Default|GetAnimationComponent)) "/Game/Character/animaciones_Ufologo/AnimSequences/Ataque.Ataque" "DefaultSlot" 1.0 0.0
      (:then
        (Variables|Default|SetEstáAtacando? true))
      (:OnCompleted
        (Variables|Default|SetEstáAtacando? false :!label _label))
      (:OnCancelled
        (goto _label)))))

(event Input|EnhancedActionEvents|EnhancedInputActionIA_SalirDeljuego
  (params (ActionValue :type Boolean) (ElapsedSeconds :type Float%20%28double-precision%29) (TriggeredSeconds :type Float%20%28double-precision%29) (InputAction :type Input%20Action%20Object%20Reference :default "/Game/Imputs/IA_SalirDeljuego.IA_SalirDeljuego"))
  ;[1 1 1] salir del juego
  (Game|QuitGame 0 "Quit" false))

(event Input|EnhancedActionEvents|EnhancedInputActionIA_AtaqueDistancia
  (params (ActionValue :type Boolean) (ElapsedSeconds :type Float%20%28double-precision%29) (TriggeredSeconds :type Float%20%28double-precision%29) (InputAction :type Input%20Action%20Object%20Reference :default "/Game/Imputs/IA_AtaqueDistancia.IA_AtaqueDistancia"))
  (bind _returnvalue (Transformation|GetActorLocation))
  (bind _returnvalue_2 (Transformation|GetActorForwardVector))
  (bind _returnvalue_3 (Transformation|GetActorTransform))
  (bind _veldash (Variables|Default|Getveldash))
  (bind _returnvalue_4 (* _returnvalue_2 _veldash))
  ;[1 1 1] Ataque distancia
  (:Started
    (if (not (Variables|Default|GetDashActivado?))
      (if (not (Variables|Default|GetEstáAtacando?))
        (Class|KismetSystemLibrary|LineTraceMultiforObjects _returnvalue (+ _returnvalue (Math|Vector|MakeVector (.x _returnvalue_4) (.y _returnvalue_4) 0.0)) (Utilities|Array|MakeArray "ObjectTypeQuery1" "ObjectTypeQuery2" "ObjectTypeQuery7") false 0 "None" true)
        (|PlayAnimationOverridewithCallbacks (Variables|/Script/PaperZD.PaperZDAnimationComponent|GetAnimInstance (Variables|Default|GetAnimationComponent)) "/Game/Character/animaciones_Ufologo/AnimSequences/AtaqueDistancia.AtaqueDistancia" "DefaultSlot" 1.0 0.0
          (:then
            (Variables|Default|SetEstaDisparando true)
            (Game|SpawnActorfromClass "/Game/Character/animaciones_Ufologo/Ataquedistancia/BP_Flecha.BP_Flecha_C" (Math|Transform|MakeTransform (Math|Vector|MakeVector (.x (.location _returnvalue_3)) (- (.y (.location _returnvalue_3)) 1e+02) (.z (.location _returnvalue_3))) (.rotation _returnvalue_3) (.scale _returnvalue_3)) "Undefined" "MultiplyWithRoot" 0 0))
          (:OnCompleted
            (Variables|Default|SetEstaDisparando false :!label _label))
          (:OnCancelled
            (goto _label)))))))

(event EventBeginPlay
  (|CallParentFunction)
  ;[1 1 1] mapeado del control añadido
  (CallFunction|AddMapping)
  (CallFunction|CreateHud))

(event Collision|EventActorBeginOverlap
  (params (OtherActor :type Actor%20Object%20Reference)))

(event EventObtenerGemas
  (params (Gemas :type Integer))
  ;[1 1 1] Gemas
  (bind _output_get (Variables|Default|SetGemas (+ Gemas (Variables|Default|GetGemas))))
  (Development|PrintString (Utilities|String|Append "Gemas" (Utilities|String|ToString(Integer) _output_get)) true true "(R=1.000000,G=0.000000,B=0.000000,A=1.000000)" 5.0))

(event EventTick
  (params (DeltaSeconds :type Float%20%28single-precision%29)))

(event EventAgarrarUnItem
  (params (item :type BP%20Item%20Object%20Reference)))

(event EventAlertaDaño
  (params (Vida :type Float%20%28double-precision%29) (VidaMaxima :type Float%20%28double-precision%29))
  ;[1 1 1] Se actualiza el daño en Hud
  (Default|Actualizarbarravida (Variables|Default|GetHUD) Vida VidaMaxima))

(event EventFlechazo)

(event EventVidaAlIniciar
  (params (Vida :type Float%20%28double-precision%29) (VidaMaxima :type Float%20%28double-precision%29))
  ;[1 1 1] Vida Al Iniciar
  (CallFunction|ActualizarWidgetVida Vida VidaMaxima))

(event EventCurarseenescenario
  (params (vida :type Float%20%28double-precision%29) (vidaMaxima :type Float%20%28double-precision%29))
  ;[1 1 1] curación reflejada en hud
  (CallFunction|ActualizarWidgetVida vida vidaMaxima))

(event EventEspadazo
  ;[1 1 1] aplica el daño segun animación de ataque cuerpo a cuerpo
  (for _array_element (Collision|GetOverlappingActors (Variables|Default|GethitBox) "/Game/Character/Enemigos/BP_EnemigorBase.BP_EnemigorBase_C" :!class /Script/Engine.PrimitiveComponent)
    (Game|Damage|ApplyDamage _array_element (Variables|Default|GetDañoDeAtaqueMele) 0 0)))

(event EventObtenerMonedas
  (params (Monedas :type Integer))
  ;[1 1 1] Monedas
  (bind _output_get (Variables|Default|SetMonedas (+ Monedas (Variables|Default|GetMonedas))))
  (Development|PrintString (Utilities|String|Append "Monedas" (Utilities|String|ToString(Integer) _output_get)) true true "(R=1.000000,G=0.000000,B=0.000000,A=1.000000)" 5.0))

(event Input|KeyboardEvents|DebugKeyT
  (params (Key :type Key%20Structure :default "None") (ActionValue :type Input%20Action%20Value%20Structure)))

(event Input|KeyboardEvents|DebugKeyM
  (params (Key :type Key%20Structure :default "None") (ActionValue :type Input%20Action%20Value%20Structure))
  (bind _bpc_componentesalud (Variables|Default|GetBPC_ComponenteSalud))
  (:Released
    (bind _output_get (Variables|Default|SetSaveEstructura (Utilities|Struct|MakeS_Save (Variables|/Game/Componentes/BPC_ComponenteSalud.BPC_ComponenteSalud_C|GetVida _bpc_componentesalud) (Variables|/Game/Componentes/BPC_ComponenteSalud.BPC_ComponenteSalud_C|GetVidaMaxima _bpc_componentesalud) 1e+01 3 "" (Transformation|GetActorTransform) 0.0 0.0 "0001.01.01-00.00.00" false)))
    (bind _asbp_giplayer (Utilities|Casting|CastToBP_GIPlayer (Game|GetGameInstance)))
    (Default|SaveGame _asbp_giplayer (Variables|Default|GetSaveEstructura))
    (Development|PrintString (Utilities|String|ToString(Transform) (.posición _output_get)) true true "(R=0.000000,G=0.660000,B=1.000000,A=1.000000)" 1e+01)))

(event Input|KeyboardEvents|DebugKeyN
  (params (Key :type Key%20Structure :default "None") (ActionValue :type Input%20Action%20Value%20Structure))
  (:Released
    (bind _asbp_giplayer (Utilities|Casting|CastToBP_GIPlayer (Game|GetGameInstance)))
    (bind _struct (Default|GetSave _asbp_giplayer))
    (bind _output_get (Variables|Default|SetSaveEstructura _struct))
    (Development|PrintString (Utilities|String|ToString(Transform) (.posición _output_get)))
    (Transformation|SetActorTransform (.posición _output_get))))

(fn ConstructionScript)

(fn CreateHud
  (bind _asplayer_controller (Utilities|Casting|CastToPlayerController (Pawn|GetController)))
  (bind _returnvalue (UserInterface|CreateWidget "/Game/UI/WBP_HUD.WBP_HUD_C" _asplayer_controller))
  (UserInterface|Viewport|AddtoViewport _returnvalue 0)
  (bind _output_get (Variables|Default|SetHUD _returnvalue))
  (Progress|SetPercent (Variables|/Game/UI/WBP_BarraDeSalud.WBP_BarraDeSalud_C|GetProgressBar (Variables|/Game/UI/WBP_HUD.WBP_HUD_C|GetWBP_BarraDeSalud _output_get)) (/ (Variables|Default|GetVida) (Variables|Default|GetSalud%20Máxima)))
  (Variables|/Script/UMG.TextBlock|SetText (Variables|/Game/UI/WBP_BarraDeSalud.WBP_BarraDeSalud_C|Getvida (Variables|/Game/UI/WBP_HUD.WBP_HUD_C|GetWBP_BarraDeSalud _output_get)) (Utilities|Text|ToText(Float) (Variables|Default|GetVida) "HalfToEven"))
  (Variables|/Script/UMG.TextBlock|SetText (Variables|/Game/UI/WBP_BarraDeSalud.WBP_BarraDeSalud_C|Getvidamáxima (Variables|/Game/UI/WBP_HUD.WBP_HUD_C|GetWBP_BarraDeSalud _output_get)) (Utilities|Text|ToText(Float) (Variables|Default|GetSalud%20Máxima) "HalfToEven")))

(fn AddMapping
  (bind _asplayer_controller (Utilities|Casting|CastToPlayerController (Pawn|GetController)))
  (Input|AddMappingContext (PlayerController|LocalPlayerSubsystems|GetEnhancedInputLocalPlayerSubsystem _asplayer_controller) "/Game/IMC_Ovnitorco.IMC_Ovnitorco" 0 "(bIgnoreAllPressedKeysUntilRelease=True,bForceImmediately=False,bNotifyUserSettings=False)"))

(fn ActualizarWidgetVida
  (params (vida :type Float%20%28double-precision%29) (vida%20máxima :type Float%20%28double-precision%29))
  (bind _hud (Variables|Default|GetHUD))
  (bind _wbp_barradesalud (Variables|/Game/UI/WBP_HUD.WBP_HUD_C|GetWBP_BarraDeSalud _hud))
  (Progress|SetPercent (Variables|/Game/UI/WBP_BarraDeSalud.WBP_BarraDeSalud_C|GetProgressBar _wbp_barradesalud) (/ vida vida%20máxima))
  (Variables|/Script/UMG.TextBlock|SetText (Variables|/Game/UI/WBP_BarraDeSalud.WBP_BarraDeSalud_C|Getvida _wbp_barradesalud) (Utilities|Text|ToText(Float) vida "HalfToEven"))
  (Variables|/Script/UMG.TextBlock|SetText (Variables|/Game/UI/WBP_BarraDeSalud.WBP_BarraDeSalud_C|Getvidamáxima _wbp_barradesalud) (Utilities|Text|ToText(Float) vida%20máxima "HalfToEven")))

(fn DañoRecibido
  (params (Daño :type Float%20%28double-precision%29))
  (bind _output_get (Variables|Default|SetVida (Math|Float|Clamp(Float) (- (Variables|Default|GetVida) Daño) 0.0 (Variables|Default|GetSalud%20Máxima))))
  (Development|PrintString (Utilities|String|ToString(Float) _output_get))
  (CallFunction|ActualizarWidgetVida 0.0 0.0))

(fn Curar
  (params (cura :type Float%20%28double-precision%29))
  (bind _output_get (Variables|Default|SetVida (Math|Float|Clamp(Float) (+ (Variables|Default|GetVida) cura) 0.0 (Variables|Default|GetSalud%20Máxima))))
  (Development|PrintString (Utilities|String|ToString(Float) _output_get))
  (CallFunction|ActualizarWidgetVida 0.0 0.0))

(fn LoadGameCharacter
  (params (struct :type S%20Save%20Structure))
  (bind _output_get (Variables|Default|SetSaveEstructura struct))
  (Variables|Default|SetVida (.vidaactual _output_get))
  (Variables|Default|SetSalud%20Máxima (.vidamax _output_get))
  (Transformation|SetActorTransform (.posición _output_get)))