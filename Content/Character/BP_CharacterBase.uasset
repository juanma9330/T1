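; Base character Blueprint that gives characters health, damage and healing logic.
; AnyDamage passes damage to the BPCComponenteSalud health component, whose life-lowered event is bound on BeginPlay to ActualizarLaVida, left empty here.
; RecibirDaño and Curarse separately adjust the character's own Vida variable, clamped between zero and SaludMáxima, without going through the component.
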(event `self.ReceiveBeginPlay`
  (add `/Game/Componentes/BPC_ComponenteSalud.SeBajóLavida` (`self.BPC_ComponenteSalud`) (delegate `ActualizarLaVida`)))

(event `ActualizarLaVida`
  (params (Vida :type "Float (double-precision)") (VidaMaxima :type "Float (double-precision)")))

(event `self.ReceiveAnyDamage`
  (params (Damage :type "Float (single-precision)") (DamageType :type "DamageType Object Reference") (InstigatedBy :type "Controller Object Reference") (DamageCauser :type "Actor Object Reference"))
  (`/Game/Componentes/BPC_ComponenteSalud.DisminuirVida` (`self.BPC_ComponenteSalud`) Damage))

(fn `Curarse`
  (params (cura :type "Float (double-precision)"))
  (set `self.Vida` (`KismetMathLibrary.FClamp` (+ (`self.Vida`) cura) 0.0 (`self.Salud Máxima`))))

(fn `RecibirDaño`
  (params (`Daño` :type "Float (double-precision)"))
  (set `self.Vida` (`KismetMathLibrary.FClamp` (- (`self.Vida`) `Daño`) 0.0 (`self.Salud Máxima`))))

(fn `UserConstructionScript`)