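; BP_ParedPuzzle is a puzzle wall that visually reflects how many gems the player's BP_Ufologo carries.
; When the Ufologo overlaps the Int component, the wall swaps its Paper2D sprite to match one, two or three gems.
; Only the three-gem case adds to GemasEnPared, sends that total to Pared through CantidadGemasenParedMessage and prints it.
; The gem addition has no guard, so repeated overlaps keep increasing the total.
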(event `self.ReceiveActorBeginOverlap`
  (params (OtherActor :type "Actor Object Reference")))

(event `self.int.OnComponentBeginOverlap`
  (params (OverlappedComponent :type "PrimitiveComponent Object Reference") (OtherActor :type "Actor Object Reference") (OtherComp :type "PrimitiveComponent Object Reference") (OtherBodyIndex :type Integer) (bFromSweep :type Boolean) (SweepResult :type "HitResult Structure (by ref)"))
  (bind _papersprite (`self.PaperSprite`))
  (bind _asbp_ufologo (cast `/Game/Character/BP_Ufologo` OtherActor))
  (bind _gemas (`/Game/Character/BP_Ufologo.Gemas` _asbp_ufologo))
  (if (== _gemas 0)
    _
    (elif (== _gemas 1)
      (`PaperSpriteComponent.SetSprite` _papersprite "/Game/Assets/Puzle/Pared1Gema_Sprite_0.Pared1Gema_Sprite_0")
      (elif (== _gemas 2)
        (`PaperSpriteComponent.SetSprite` _papersprite "/Game/Assets/Puzle/Pared2Gema_Sprite_0.Pared2Gema_Sprite_0")
        (elif (== _gemas 3)
          (`PaperSpriteComponent.SetSprite` _papersprite "/Game/Assets/Puzle/Pared3Gema_Sprite_0.Pared3Gema_Sprite_0")
          (bind _output_get (set `self.GemasEnPared` (+ (`self.GemasEnPared`) 3)))
          (message `/Game/Interfases/BPI_GemasPared.cantidadGemasenPared` (`self.Pared`) _output_get)
          (`KismetSystemLibrary.PrintString` (`KismetStringLibrary.Concat_StrStr` "GEMAS EN PARED" (`KismetStringLibrary.Conv_IntToString` _output_get))))))))

(event `Cambioskin`)

(fn `UserConstructionScript`)